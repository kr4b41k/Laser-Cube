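; AI chicken that ages, tracks hunger, thirst, stamina and egg-laying urge, and dies from damage into a ragdoll with sound and feathers.
; A looping timer updates stats, scales body and material by age, and writes need flags to the Blackboard.
; ScareTrigger overlaps with tagged actors repeatedly set a navigable flee location.
; Startled or damaged chickens temporarily take the scare tag themselves, spreading panic to others.
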(event OnComponentBeginOverlap(ScareTrigger)
  (params (OverlappedComponent :type Primitive%20Component%20Object%20Reference) (OtherActor :type Actor%20Object%20Reference) (OtherComp :type Primitive%20Component%20Object%20Reference) (OtherBodyIndex :type Integer) (bFromSweep :type Boolean) (SweepResult :type Hit%20Result%20Structure%20%28by%20ref%29))
  (bind _returnvalue (Pawn|GetController))
  (bind _tag_to_scare_chicken (Variables|Flee|GetTag%20to%20scare%20chicken))
  (bind _returnvalue_2 (AI|GetBlackboard _returnvalue))
  ;[0 0 0] Actor to flee from enters "ScareTrigger"
  (if (not (Variables|Flee|GetShould%20flee?))
    (if (or (Components|ComponentHasTag OtherComp _tag_to_scare_chicken) (Actor|ActorHasTag OtherActor _tag_to_scare_chicken))
      (Variables|Flee|SetShould%20flee? true)
      (Variables|Flee|SetActor%20to%20flee%20from OtherActor)
      (CallFunction|ScareOtherChickens 0.5)
      (AI|Components|Blackboard|SetValueasVector _returnvalue_2 (Utilities|Name|MakeLiteralName "FleeLocation") (|CalcFleeLocation))
      (AI|Components|Blackboard|SetValueasBool _returnvalue_2 (Utilities|Name|MakeLiteralName "Flee?") true)
      (Utilities|FlowControl|Delay 0.01)
      (CallFunction|RepeatFlee)
      (Variables|Stats|SetResting? false)
      ;[1 0 0.7297] Cosmetic particles
      (Utilities|FlowControl|DoOnce false
        (:Completed
          (if (> (.Statvalue (Utilities|Struct|BreakStructStat (Variables|Stats|GetAge))) 8e+01)
            (Effects|SpawnEmitterAttached "/Game/ChickenAI/Demo/Particles/P_FeatherDrop.P_FeatherDrop" (Variables|Character|GetMesh) "Chest" "0, 0, 0" "0, 0, 0" "1.000000,1.000000,1.000000" "SnapToTargetIncludingScale")))))))

(event OnComponentEndOverlap(ScareTrigger)
  (params (OverlappedComponent :type Primitive%20Component%20Object%20Reference) (OtherActor :type Actor%20Object%20Reference) (OtherComp :type Primitive%20Component%20Object%20Reference) (OtherBodyIndex :type Integer))
  (bind _returnvalue (Pawn|GetController))
  (bind _returnvalue_2 (AI|GetBlackboard _returnvalue))
  ;[0 0 0] Actor to flee exits "ScareTrigger"
  (if (Variables|Flee|GetShould%20flee?)
    (if (== OtherActor (Variables|Flee|GetActor%20to%20flee%20from))
      (Utilities|IsValid _returnvalue_2
        (:Is%20Valid
          (AI|Components|Blackboard|SetValueasBool _returnvalue_2 (Utilities|Name|MakeLiteralName "Flee?") false)
          (Variables|Flee|SetShould%20flee? false)
          ;[1 0 0.7297] Cosmetic particles
          (Utilities|FlowControl|DoOnce false) ; enters at Reset
        )))))

(event Custom|Toggle%20Debug
  (params (Debug%20on? :type Boolean))
  ;[1 0 0.6047] Toggle debug
  (Default|Show/HideDebug (Variables|Debug|GetDebugWidget) Debug%20on?))

(event Custom|Repeat%20flee
  (bind _returnvalue (Pawn|GetController))
  (bind _returnvalue_2 (AI|GetBlackboard _returnvalue))
  ;[0 0 0] Actor to flee from enters "ScareTrigger"
  (if (Variables|Flee|GetShould%20flee?)
    (AI|Components|Blackboard|SetValueasVector _returnvalue_2 (Utilities|Name|MakeLiteralName "FleeLocation") (|CalcFleeLocation))
    (AI|Components|Blackboard|SetValueasBool _returnvalue_2 (Utilities|Name|MakeLiteralName "Flee?") true)
    (Utilities|FlowControl|Delay 0.01)
    (CallFunction|RepeatFlee)
    (Variables|Stats|SetResting? false)
    ;[1 0 0.7297] Cosmetic particles
    (Utilities|FlowControl|DoOnce false
      (:Completed
        (if (> (.Statvalue (Utilities|Struct|BreakStructStat (Variables|Stats|GetAge))) 8e+01)
          (Effects|SpawnEmitterAttached "/Game/ChickenAI/Demo/Particles/P_FeatherDrop.P_FeatherDrop" (Variables|Character|GetMesh) "Chest" "0, 0, 0" "0, 0, 0" "1.000000,1.000000,1.000000" "SnapToTargetIncludingScale"))))))

(event Custom|Start%20resting
  ;[0 0 0] Start resting
  (Variables|Stats|SetResting? true))

(event Custom|Scare%20other%20chickens
  (params (How%20long? :type Float%20%28single-precision%29))
  (bind _tags (Variables|Actor|GetTags))
  (bind _tag_to_scare_chicken (Variables|Flee|GetTag%20to%20scare%20chicken))
  (bind _mesh (Variables|Character|GetMesh))
  (bind _componenttags (Variables|/Script/Engine.ActorComponent|GetComponentTags _mesh))
  ;[0 0 0] Scare other chickens when startled
  (Utilities|Array|AddUnique _tags _tag_to_scare_chicken)
  (Utilities|Array|AddUnique _componenttags _tag_to_scare_chicken)
  (Utilities|FlowControl|RetriggerableDelay How%20long?)
  (Utilities|Array|RemoveItem _tags _tag_to_scare_chicken)
  (Utilities|Array|RemoveItem _componenttags _tag_to_scare_chicken))

(event Game|Damage|EventAnyDamage
  (params (Damage :type Float%20%28single-precision%29) (DamageType :type Damage%20Type%20Object%20Reference) (InstigatedBy :type Controller%20Object%20Reference) (DamageCauser :type Actor%20Object%20Reference))
  ;[0 0 0] Damage & Death
  (CallFunction|ScareOtherChickens 5.0)
  (if (Variables|Stats|GetDead?)
    (Utilities|FlowControl|DoN 2 ; Drop feathers after death
      (:Exit
        ;[1 0 0.8197] Death particles
        (if (> (.Statvalue (Utilities|Struct|BreakStructStat (Variables|Stats|GetAge))) 8e+01) :!label _label
          (Effects|SpawnEmitterAttached "/Game/ChickenAI/Demo/Particles/P_FeatherExplosion.P_FeatherExplosion" (Variables|Character|GetMesh) "Chest" "0, 0, 0" "0, 0, 0" "1.000000,1.000000,1.000000" "SnapToTargetIncludingScale"))))
    (else
      (bind _output_get (Variables|Stats|SetHealth (- (Variables|Stats|GetHealth) Damage)))
      (if (<= _output_get 0.0)
        (Variables|Stats|SetDead? true)
        (Utilities|Time|ClearTimerbyFunctionName 0 "Update stats")
        (Components|DestroyComponent (Variables|Collision|GetCapsuleComponent))
        (bind _returnvalue (Audio|SpawnSoundatLocation "/Game/ChickenAI/Demo/Sound/Chicken_Death_Cue.Chicken_Death_Cue" (Transformation|GetActorLocation) "0, 0, 0" 1.0 1.0 0.0 0 0))
        (Audio|Components|Audio|SetPitchMultiplier _returnvalue (|Calculatepitchbysize))
        (Components|Animation|SetAnimationMode (Variables|Character|GetMesh) "AnimationCustomMode")
        (Physics|SetSimulatePhysics (Variables|Character|GetMesh) true)
        (goto _label)))))

(event EventBeginPlay
  ;[0 0 0] Initialize stats timer
  (Utilities|Time|SetTimerbyFunctionName 0 "Update stats" (Variables|Stats|GetTime%20to%20update%20stats) true)
  ;[0 0 0] Randomize gender
  (if (Variables|Stats|GetRandomize%20gender?)
    (Variables|Stats|SetFemale? (Math|Random|RandomBool)))
  ;[1 0 0.4947] Save debug widget to variable
  (bind _asdebug_widget (Utilities|Casting|CastToDebugWidget (UserInterface|GetUserWidgetObject (Variables|Default|GetDebug%20Widget))))
  (Variables|Debug|SetDebugWidget _asdebug_widget)
  ;[1 0 0.8061] Initialize debug
  (bind _asfirst_person_character (Utilities|Casting|CastToFirstPersonCharacter (Game|Player|GetPlayerPawn 0)))
  (CallFunction|ToggleDebug (Variables|/Game/ChickenAI/Demo/UnrealContent/FirstPersonBP/Blueprints/FirstPersonCharacter.FirstPersonCharacter_C|GetDebug _asfirst_person_character)))

(fn ConstructionScript
  (bind _age (Variables|Stats|GetAge))
  (bind _statvalue (Utilities|Struct|BreakStructStat _age))
  (Transformation|SetRelativeScale3D (Variables|Character|GetMesh) (Math|Conversions|ToVector(Float) (Math|Float|MapRangeClamped _statvalue 0.0 1e+02 0.4 1.0)))
  (Components|Capsule|SetCapsuleRadius (Variables|Collision|GetCapsuleComponent) (Math|Float|MapRangeClamped _statvalue 0.0 1e+02 5.0 15.0) true)
  (bind _returnvalue (Rendering|Material|CreateDynamicMaterialInstance (Variables|Character|GetMesh) 0 "/Game/ChickenAI/Demo/Materials/Chicken/MI_ChickenWhite.MI_ChickenWhite" "None" :!class /Script/Engine.PrimitiveComponent))
  (bind _output_get (Variables|Cosmetic|SetChicken%20material _returnvalue))
  (Rendering|Material|SetScalarParameterValue _output_get "Age" (Math|Float|MapRangeClamped (.Statvalue (Utilities|Struct|BreakStructStat (Variables|Stats|GetAge))) 0.0 1e+02 0.0 1.0) :!class /Script/Engine.MaterialInstanceDynamic))

(fn UpdateStats
  (if (not (Variables|Stats|GetDead?))
    (Variables|Stats|SetStamina (Utilities|Struct|MakeStructStat (Math|Float|Clamp(Float) (+ (.Statvalue (Utilities|Struct|BreakStructStat (Variables|Stats|GetStamina))) (Math|Float|SelectFloat (Variables|Stats|GetStamina%20increase%20per%20update%20when%20resting) (.Changeperupdate (Utilities|Struct|BreakStructStat (Variables|Stats|GetStamina))) (Variables|Stats|GetResting?))) 0.0 1e+02) (.Changeperupdate (Utilities|Struct|BreakStructStat (Variables|Stats|GetStamina)))))
    (Variables|Stats|SetHunger (Utilities|CalculateStatUpdate (Variables|Stats|GetHunger)))
    (Variables|Stats|SetThirst (Utilities|CalculateStatUpdate (Variables|Stats|GetThirst)))
    (Variables|Stats|SetUrge%20to%20lay%20egg (select (and (Variables|Stats|GetFemale?) (> (.Statvalue (Utilities|Struct|BreakStructStat (Variables|Stats|GetAge))) 8e+01)) (Utilities|CalculateStatUpdate (Variables|Stats|GetUrge%20to%20lay%20egg)) (|Nullegglaying (Utilities|CalculateStatUpdate (Variables|Stats|GetUrge%20to%20lay%20egg)))))
    (Variables|Stats|SetAge (Utilities|CalculateStatUpdate (Variables|Stats|GetAge)))
    (|Changebodybyage)
    (|Updateblackboardvalues) ; Update blackboard values
    ;[1 0 0.9235] Update debug widget
    (Default|UpdateWidget (Variables|Debug|GetDebugWidget) (Variables|Stats|GetFemale?) (.Statvalue (Utilities|Struct|BreakStructStat (Variables|Stats|GetAge))) (.Statvalue (Utilities|Struct|BreakStructStat (Variables|Stats|GetHunger))) (.Statvalue (Utilities|Struct|BreakStructStat (Variables|Stats|GetThirst))) (.Statvalue (Utilities|Struct|BreakStructStat (Variables|Stats|GetStamina))) (.Statvalue (Utilities|Struct|BreakStructStat (Variables|Stats|GetUrge%20to%20lay%20egg))))))