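; Default pawn that lets the player rotate a mirror, apparently for a laser puzzle, while a mirror prompt widget is active.
; DPSTR and DPEND store the sending object and show or hide the widget, toggling rotation, though first-time widget creation leaves the flag unset.
; Two input actions call angle helpers, send the result to that sender via SetRotationMessage and play a sound.
; The helpers' clamped 45-degree math and most of CallWBStart are unconnected.
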(event Input|EnhancedActionEvents|EnhancedInputActioneeeee
  (params (ActionValue :type Boolean) (ElapsedSeconds :type Float%20%28double-precision%29) (TriggeredSeconds :type Float%20%28double-precision%29) (InputAction :type Input%20Action%20Object%20Reference :default "/AscentCombatFramework/Input/eeeee.eeeee"))
  (if (Variables|Default|GetCanRotateMirror)
    (bind _output_get (Variables|Default|SetRotateAngle (|PlusAngle)))
    (Class|BPIMirror|SetRotation(Message) (Variables|Default|GetSender) _output_get)
    (Audio|PlaySound2D "/Game/BluePrints/Sounds/LaserTarget.LaserTarget" 0.1 1.0 0.1 0 0)))

(event Input|EnhancedActionEvents|EnhancedInputActionqqqq
  (params (ActionValue :type Boolean) (ElapsedSeconds :type Float%20%28double-precision%29) (TriggeredSeconds :type Float%20%28double-precision%29) (InputAction :type Input%20Action%20Object%20Reference :default "/AscentCombatFramework/Input/qqqq.qqqq"))
  (if (Variables|Default|GetCanRotateMirror)
    (bind _output_get (Variables|Default|SetRotateAngle (|SubstructAngle)))
    (Class|BPIMirror|SetRotation(Message) (Variables|Default|GetSender) _output_get)
    (Audio|PlaySound2D "/Game/BluePrints/Sounds/LaserTarget.LaserTarget" 0.1 1.0 0.1 0 0)))

(event EventBeginPlay
  (|CallParentFunction) ; This node is disabled and will not be called.\nDrag off pins to build functionality.
)

(event Collision|EventActorBeginOverlap
  (params (OtherActor :type Actor%20Object%20Reference))
  (|CallParentFunction OtherActor) ; This node is disabled and will not be called.\nDrag off pins to build functionality.
)

(event EventTick
  (params (DeltaSeconds :type Float%20%28single-precision%29))
  (|CallParentFunction DeltaSeconds) ; This node is disabled and will not be called.\nDrag off pins to build functionality.
)

(event EventDPEND
  (params (Sender :type Actor%20Object%20Reference))
  (Variables|Default|SetSender Sender)
  (Widget|SetVisibility (Variables|Default|GetWidgetMirror) "Hidden")
  (Variables|Default|SetCanRotateMirror false))

(event EventDPSTR
  (params (Sender :type Actor%20Object%20Reference))
  (Variables|Default|SetSender Sender)
  (Utilities|IsValid (Variables|Default|GetWidgetMirror)
    (:Is%20Valid
      (Widget|SetVisibility (Variables|Default|GetWidgetMirror) "Visible")
      (Variables|Default|SetCanRotateMirror true))
    (:Is%20Not%20Valid
      (bind _returnvalue (UserInterface|CreateWidget "/Game/BluePrints/LevelLogicMechanicks/Base_Logic/Mirror/WB_Mirror.WB_Mirror_C" (Game|GetPlayerController 0)))
      (bind _output_get (Variables|Default|SetWidgetMirror _returnvalue))
      (UserInterface|Viewport|AddtoViewport _output_get 0))))

(fn ConstructionScript
  (|CallParentFunction))

(fn CallWBEnd
  (Widget|SetVisibility (Variables|Default|GetWidgetMirror) "Hidden")
  (Variables|Default|SetCanRotateMirror false)
  (return true))

(fn CallWBStart
  (params (Sender :type Actor%20Object%20Reference))
  (Variables|Default|SetSender Sender))