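; Default pawn that lets the player activate button points and open dialogs with the E key.
; Interface calls from a button point store the sender and dialog flag, then show or hide a reused prompt widget.
; Releasing E either sends a press message to that point, gated by CanPressButtonPoint, or opens its dialog text in a UI-only widget with sounds.
; The cube and generic widget interface calls are empty stubs.
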(event EventBeginPlay
  (|CallParentFunction) ; This node is disabled and will not be called.\nDrag off pins to build functionality.
)

(event Collision|EventActorBeginOverlap
  (params (OtherActor :type Actor%20Object%20Reference))
  (|CallParentFunction OtherActor) ; This node is disabled and will not be called.\nDrag off pins to build functionality.
)

(event EventTick
  (params (DeltaSeconds :type Float%20%28single-precision%29))
  (|CallParentFunction DeltaSeconds) ; This node is disabled and will not be called.\nDrag off pins to build functionality.
)

(event Input|KeyboardEvents|E
  (params (Key :type Key%20Structure :default "None"))
  (:Released
    (if (Variables|Default|GetIs%20Dialog?)
      (bind _description (Class|BPIABaseDialog|GetDialogText(Message) (Variables|Default|GetLO_ButtonPoint)))
      (bind _returnvalue (UserInterface|CreateWidget "/Game/BluePrints/LevelLogicMechanicks/Base_Logic/Dialog/WBP/WB_Dialog.WB_Dialog_C" 0 _description))
      (Variables|/Script/Engine.PlayerController|SetbShowMouseCursor (Game|GetPlayerController 0) true)
      (Input|SetInputModeUIOnly (Game|GetPlayerController 0) _returnvalue "DoNotLock" false)
      (Class|BPIPCWidgetControll|PCAddWidget(Message) (Game|GetPlayerController 0) _returnvalue)
      (Audio|PlaySound2D "/Game/BluePrints/Sounds/RobotTalk.RobotTalk" 0.2 0.8 0.0 0 0)
      (Audio|PlaySound2D "/Game/BluePrints/Sounds/LaserTarget.LaserTarget" 1.0 1.0 0.0 0 0)
      (elif (Variables|Default|GetCanPressButtonPoint)
        (Class|BPIButtonPoint|PressButtonPoint(Message) (Variables|Default|GetLO_ButtonPoint))))))

(fn ConstructionScript
  (|CallParentFunction))

(fn CallWBCubeStart
  (return false))

(fn CallWBCubeEnd
  (return false))

(fn CallWBEnd
  (return false))

(fn CallWBStart
  (params (Sender :type Actor%20Object%20Reference))
  (return false))

(fn CallWBButtonPointEnd
  (params (IsDialog? :type Boolean))
  (Variables|Default|SetIs%20Dialog? IsDialog?)
  (Utilities|IsValid (Variables|Default|GetWB_ButtonPoint)
    (:Is%20Valid
      (Widget|SetVisibility (Variables|Default|GetWB_ButtonPoint) "Hidden")
      (Variables|Default|SetCanPressButtonPoint false)
      (return true))))

(fn CallWBButtonPointStart
  (params (Sender :type Actor%20Object%20Reference) (is_dialog? :type Boolean))
  (Variables|Default|SetIs%20Dialog? is_dialog?)
  (Variables|Default|SetLO_ButtonPoint Sender)
  (Utilities|IsValid (Variables|Default|GetWB_ButtonPoint)
    (:Is%20Valid
      (Widget|SetVisibility (Variables|Default|GetWB_ButtonPoint) "Visible")
      (Variables|Default|SetCanPressButtonPoint true))
    (:Is%20Not%20Valid
      (bind _returnvalue (UserInterface|CreateWidget "/Game/BluePrints/LevelLogicMechanicks/Base_Logic/Button(Point)/WB_ButtonPoint.WB_ButtonPoint_C"))
      (bind _output_get (Variables|Default|SetWB_ButtonPoint _returnvalue))
      (UserInterface|Viewport|AddtoViewport _output_get 0)
      (return true))))