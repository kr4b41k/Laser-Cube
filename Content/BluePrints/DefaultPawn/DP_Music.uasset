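; DP_Music is a pawn that plays the MS_GameAmbient sound in 2D on BeginPlay and contains camera-shift logic driven by sphere overlaps.
; Sphere begin overlap requests a looping CameraEvent timer with zero interval, which Unreal does not schedule, and end overlap clears the handle.
; CameraEvent is written to nudge the SpringArm socket offset one unit along Y per call, with no limit or reset.
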(event OnComponentBeginOverlap(Sphere)
  (params (OverlappedComponent :type Primitive%20Component%20Object%20Reference) (OtherActor :type Actor%20Object%20Reference) (OtherComp :type Primitive%20Component%20Object%20Reference) (OtherBodyIndex :type Integer) (bFromSweep :type Boolean) (SweepResult :type Hit%20Result%20Structure%20%28by%20ref%29))
  (bind _returnvalue (Utilities|Time|SetTimerbyEvent (delegate Custom|CameraEvent) 0.0 true))
  (Variables|Default|SetCameraTimer _returnvalue))

(event OnComponentEndOverlap(Sphere)
  (params (OverlappedComponent :type Primitive%20Component%20Object%20Reference) (OtherActor :type Actor%20Object%20Reference) (OtherComp :type Primitive%20Component%20Object%20Reference) (OtherBodyIndex :type Integer))
  (Utilities|Time|ClearandInvalidateTimerbyHandle (Variables|Default|GetCameraTimer)))

(event Custom|CameraEvent
  (bind _springarm (Variables|Default|GetSpringArm))
  (Variables|/Script/Engine.SpringArmComponent|SetSocketOffset _springarm (Math|Vector|MakeVector (.x (Variables|/Script/Engine.SpringArmComponent|GetSocketOffset _springarm)) (+ (.y (Variables|/Script/Engine.SpringArmComponent|GetSocketOffset _springarm)) 1.0) (.z (Variables|/Script/Engine.SpringArmComponent|GetSocketOffset _springarm)))))

(event EventBeginPlay
  (|CallParentFunction)
  (Audio|PlaySound2D "/Game/BluePrints/Music/MS_GameAmbient.MS_GameAmbient" 1.0 1.0 0.0 0 0))

(fn ConstructionScript
  (|CallParentFunction))