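; DP_CubeWB is a pawn Blueprint that shows and hides the WB_Cube UI widget.
; WBCStart and CallWBCubeStart lazily create the widget for player 0 on first use and re-show it afterwards, only while IsTakeable is false.
; WBCEnd and CallWBCubeEnd hide the cached widget, with the function versions returning true on success.
; CallWBStart and CallWBEnd are stubs, and Tick only calls the parent.
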(event EventBeginPlay
  (|CallParentFunction) ; This node is disabled and will not be called.\nDrag off pins to build functionality.
)

(event Collision|EventActorBeginOverlap
  (params (OtherActor :type Actor%20Object%20Reference))
  (|CallParentFunction OtherActor) ; This node is disabled and will not be called.\nDrag off pins to build functionality.
)

(event EventTick
  (params (DeltaSeconds :type Float%20%28single-precision%29))
  (|CallParentFunction DeltaSeconds))

(event EventWBCEnd
  (Utilities|IsValid (Variables|Default|GetWB_Cube)
    (:Is%20Valid
      (Widget|SetVisibility (Variables|Default|GetWB_Cube) "Hidden"))))

(event EventWBCStart
  (if (not (Variables|Default|GetIs_Takeable?))
    (Utilities|IsValid (Variables|Default|GetWB_Cube)
      (:Is%20Valid
        (Widget|SetVisibility (Variables|Default|GetWB_Cube) "Visible"))
      (:Is%20Not%20Valid
        (bind _returnvalue (UserInterface|CreateWidget "/Game/BluePrints/LevelLogicMechanicks/Base_Logic/Cube/WB_Cube.WB_Cube_C" (Game|GetPlayerController 0)))
        (bind _output_get (Variables|Default|SetWB_Cube _returnvalue))
        (UserInterface|Viewport|AddtoViewport _output_get 0)))))

(fn ConstructionScript
  (|CallParentFunction))

(fn CallWBEnd)

(fn CallWBStart
  (params (Sender :type Actor%20Object%20Reference))
  (return false))

(fn CallWBCubeEnd
  (Utilities|IsValid (Variables|Default|GetWB_Cube)
    (:Is%20Valid
      (Widget|SetVisibility (Variables|Default|GetWB_Cube) "Hidden")
      (return true))))

(fn CallWBCubeStart
  (if (not (Variables|Default|GetIs_Takeable?))
    (Utilities|IsValid (Variables|Default|GetWB_Cube)
      (:Is%20Valid
        (Widget|SetVisibility (Variables|Default|GetWB_Cube) "Visible")
        (return true))
      (:Is%20Not%20Valid
        (bind _returnvalue (UserInterface|CreateWidget "/Game/BluePrints/LevelLogicMechanicks/Base_Logic/Cube/WB_Cube.WB_Cube_C" (Game|GetPlayerController 0)))
        (bind _output_get (Variables|Default|SetWB_Cube _returnvalue))
        (UserInterface|Viewport|AddtoViewport _output_get 0)
        (return true)))))