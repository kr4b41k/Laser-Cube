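; Pawn that lets the player pick up and drop physics objects with the left mouse button.
; A click traces forward from the camera with debug drawing, grabs any simulating component via PhysicsHandle, nudges it and notifies DP_CubeWB.
; A looping timer, rather than Tick, keeps the held object at a fixed distance ahead of the camera.
; Another click releases it, with the same sound playing on grab and release.
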(event Custom|hend
  (bind _camera (Variables|Default|GetCamera))
  (if (Variables|Default|GetIs_Takeable?)
    (Physics|Components|PhysicsHandle|SetTargetLocation (Variables|Default|GetPhysicsHandle) (+ (Transformation|GetWorldLocation _camera) (* (Math|Vector|GetForwardVector _camera) 500)))))

(event EventBeginPlay
  (|CallParentFunction)
  (bind _returnvalue (Utilities|Time|SetTimerbyFunctionName 0 "Hend" 0.01 true))
  (Variables|Default|SetHandle _returnvalue))

(event Collision|EventActorBeginOverlap
  (params (OtherActor :type Actor%20Object%20Reference))
  (|CallParentFunction OtherActor) ; This node is disabled and will not be called.\nDrag off pins to build functionality.
)

(event EventTick
  (params (DeltaSeconds :type Float%20%28single-precision%29))
  (|CallParentFunction DeltaSeconds))

(event Input|MouseEvents|LeftMouseButton
  (params (Key :type Key%20Structure :default "None"))
  (bind _camera (Variables|Default|GetCamera))
  (bind _returnvalue (Transformation|GetWorldLocation _camera))
  (:Pressed
    (if (Variables|Default|GetIs_Takeable?)
      (Physics|Components|PhysicsHandle|ReleaseComponent (Variables|Default|GetPhysicsHandle))
      (Variables|Default|SetIs_Takeable? false)
      (Audio|PlaySound2D "/Game/BluePrints/Sounds/TakeCube.TakeCube" 1.0 1.0 0.0 0 0)
      (else
        (bind (_outhit _returnvalue_2) (Collision|LineTraceByChannel _returnvalue (+ _returnvalue (* (Math|Vector|GetForwardVector _camera) 1000)) "TraceTypeQuery1" false 0 "ForDuration"))
        (if _returnvalue_2
          (if (Physics|IsSimulatingPhysics (.HitComponent (Collision|BreakHitResult _outhit)) "None")
            (Class|PhysicsHandleComponent|GrabComponentatLocation (Variables|Default|GetPhysicsHandle) (.HitComponent (Collision|BreakHitResult _outhit)) "None" (Transformation|GetWorldLocation (.HitComponent (Collision|BreakHitResult _outhit))))
            (Physics|AddImpulse (.HitComponent (Collision|BreakHitResult _outhit)) "0.000000,0.100000,0.000000" "None" false)
            (Variables|Default|SetIs_Takeable? true)
            (bind _returnvalue_3 (Actor|GetActorOfClass "/Game/BluePrints/DefaultPawn/DP_CubeWB.DP_CubeWB_C"))
            (Class|BPIDPCubeWB|CallWBCubeEnd(Message) _returnvalue_3)
            (Audio|PlaySound2D "/Game/BluePrints/Sounds/TakeCube.TakeCube" 1.0 1.0 0.0 0 0)))))))

(fn ConstructionScript
  (|CallParentFunction))