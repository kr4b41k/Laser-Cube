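; DP_Main is a player pawn Blueprint that turns Enhanced Input actions into character movement and combat actions using ACF components.
; Move, sprint and crouch checks go through LocomotionComp, with sprint stepping the locomotion state up on press and resetting it on release.
; Crouch toggles, jump calls the built-in function, and melee equip triggers a highest-priority, storable action on ActionsComp.
; Escape quits the game directly.
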(event EventBeginPlay
  (|CallParentFunction))

(event Collision|EventActorBeginOverlap
  (params (OtherActor :type Actor%20Object%20Reference))
  (|CallParentFunction OtherActor) ; This node is disabled and will not be called.\nDrag off pins to build functionality.
)

(event EventTick
  (params (DeltaSeconds :type Float%20%28single-precision%29)))

(event Input|EnhancedActionEvents|EnhancedInputActionACFMoveForwardInput
  (params (ActionValue :type Float%20%28double-precision%29) (ElapsedSeconds :type Float%20%28double-precision%29) (TriggeredSeconds :type Float%20%28double-precision%29) (InputAction :type Input%20Action%20Object%20Reference :default "/AscentCombatFramework/Input/ACFMoveForwardInput.ACFMoveForwardInput"))
  (Class|ACFCharacterMovementComponent|MoveForward (Variables|Default|GetLocomotionComp) ActionValue))

(event Input|EnhancedActionEvents|EnhancedInputActionACFMoveRightInput
  (params (ActionValue :type Float%20%28double-precision%29) (ElapsedSeconds :type Float%20%28double-precision%29) (TriggeredSeconds :type Float%20%28double-precision%29) (InputAction :type Input%20Action%20Object%20Reference :default "/AscentCombatFramework/Input/ACFMoveRightInput.ACFMoveRightInput"))
  (Class|ACFCharacterMovementComponent|MoveRight (Variables|Default|GetLocomotionComp) ActionValue))

(event Input|EnhancedActionEvents|EnhancedInputActionACFSprintInput
  (params (ActionValue :type Boolean) (ElapsedSeconds :type Float%20%28double-precision%29) (TriggeredSeconds :type Float%20%28double-precision%29) (InputAction :type Input%20Action%20Object%20Reference :default "/AscentCombatFramework/Input/ACFSprintInput.ACFSprintInput"))
  (:Started
    (CallFunction|MainSprint))
  (:Completed
    (CallFunction|MainStopsprint)))

(event Input|EnhancedActionEvents|EnhancedInputActionACFCrouchInput
  (params (ActionValue :type Boolean) (ElapsedSeconds :type Float%20%28double-precision%29) (TriggeredSeconds :type Float%20%28double-precision%29) (InputAction :type Input%20Action%20Object%20Reference :default "/AscentCombatFramework/Input/ACFCrouchInput.ACFCrouchInput"))
  (if (AI|Components|NavMovement|IsCrouching (Variables|Default|GetLocomotionComp))
    (Character|UnCrouch)
    (else
      (Character|Crouch))))

(event Input|EnhancedActionEvents|EnhancedInputActionACFJumpInput
  (params (ActionValue :type Boolean) (ElapsedSeconds :type Float%20%28double-precision%29) (TriggeredSeconds :type Float%20%28double-precision%29) (InputAction :type Input%20Action%20Object%20Reference :default "/AscentCombatFramework/Input/ACFJumpInput.ACFJumpInput"))
  (Character|Jump))

(event Input|EnhancedActionEvents|EnhancedInputActionACFEquipMeleeInput
  (params (ActionValue :type Boolean) (ElapsedSeconds :type Float%20%28double-precision%29) (TriggeredSeconds :type Float%20%28double-precision%29) (InputAction :type Input%20Action%20Object%20Reference :default "/AscentCombatFramework/Input/ACFEquipMeleeInput.ACFEquipMeleeInput"))
  (Class|ACFActionsManagerComponent|TriggerAction (Variables|Default|GetActionsComp) "(TagName=\"Actions.Equip.Melee\")" "EHighest" true))

(event Input|KeyboardEvents|Escape
  (params (Key :type Key%20Structure :default "None"))
  (:Pressed
    (Game|QuitGame 0 "Quit" false)))

(fn ConstructionScript
  (|CallParentFunction))

(fn MainSprint
  (Variables|Default|SetSprint_Pressed true)
  (Class|ACFCharacterMovementComponent|AcceleratetoNextState (Variables|Default|GetLocomotionComp)))

(fn MainStopsprint
  (Variables|Default|SetSprint_Pressed false)
  (Class|ACFCharacterMovementComponent|ResettoDefaultLocomotionState (Variables|Default|GetLocomotionComp)))