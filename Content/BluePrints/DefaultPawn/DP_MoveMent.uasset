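; DP_MoveMent is a player character Blueprint that provides walking, mouse look, jumping and sprinting.
; Axis inputs move it along the actor's forward and right vectors and drive controller yaw and pitch, while Space Bar triggers Jump.
; StartSprint and FinishSprint events play and reverse a timeline that blends MaxWalkSpeed between walk and sprint speeds; nothing in this Blueprint calls them.
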(event EventBeginPlay)

(event Collision|EventActorBeginOverlap
  (params (OtherActor :type Actor%20Object%20Reference)))

(event EventTick
  (params (DeltaSeconds :type Float%20%28single-precision%29)))

(event EventStartSprint
  (bind _alpha (Timeline|SprintTimeline Play)
    (:Update
      (Variables|/Script/Engine.CharacterMovementComponent|SetMaxWalkSpeed (Variables|Character|GetCharacterMovement) (Math|Float|Lerp 6e+02 9e+02 _alpha)))))

(event EventFinishSprint
  (bind _alpha (Timeline|SprintTimeline Reverse)
    (:Update
      (Variables|/Script/Engine.CharacterMovementComponent|SetMaxWalkSpeed (Variables|Character|GetCharacterMovement) (Math|Float|Lerp 6e+02 9e+02 _alpha)))))

(event Input|AxisEvents|InputAxisFrontC
  (params (AxisValue :type Float%20%28single-precision%29))
  (Pawn|Input|AddMovementInput (Transformation|GetActorForwardVector) AxisValue false))

(event Input|AxisEvents|InputAxisRightC
  (params (AxisValue :type Float%20%28single-precision%29))
  (Pawn|Input|AddMovementInput (Transformation|GetActorRightVector) AxisValue false))

(event Input|AxisEvents|InputAxisMouseX
  (params (AxisValue :type Float%20%28single-precision%29))
  (Pawn|Input|AddControllerYawInput AxisValue))

(event Input|AxisEvents|InputAxisMouseY
  (params (AxisValue :type Float%20%28single-precision%29))
  (Pawn|Input|AddControllerPitchInput AxisValue))

(event Input|KeyboardEvents|SpaceBar
  (params (Key :type Key%20Structure :default "None"))
  (:Pressed
    (Character|Jump)))

(fn ConstructionScript)