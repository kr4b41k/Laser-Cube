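; Pawn Blueprint that lets the player pick up and drop physics objects with a left-click toggle.
; On click, a debug-drawn Visibility line trace from the camera finds a simulating component, which the PhysicsHandle grabs at its world location with a tiny impulse.
; A fast looping timer, rather than Tick, moves the handle's target to the Scene component's position while an object is held.
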(event Custom|hend
  (if (Variables|Default|GetIs_Vsat?)
    (Physics|Components|PhysicsHandle|SetTargetLocation (Variables|Default|GetPhysicsHandle) (Transformation|GetWorldLocation (Variables|Default|GetScene)))))

(event EventBeginPlay
  (|CallParentFunction)
  (bind _returnvalue (Utilities|Time|SetTimerbyFunctionName 0 "Hend" 0.01 true))
  (Variables|Default|Sethendle _returnvalue))

(event Collision|EventActorBeginOverlap
  (params (OtherActor :type Actor%20Object%20Reference))
  (|CallParentFunction OtherActor) ; This node is disabled and will not be called.\nDrag off pins to build functionality.
)

(event EventTick
  (params (DeltaSeconds :type Float%20%28single-precision%29))
  (|CallParentFunction DeltaSeconds))

(event Input|MouseEvents|LeftMouseButton
  (params (Key :type Key%20Structure :default "None"))
  (bind _camera (Variables|Default|GetCamera))
  (bind _returnvalue (Transformation|GetWorldLocation _camera))
  (:Pressed
    (if (Variables|Default|GetIs_Vsat?)
      (Physics|Components|PhysicsHandle|ReleaseComponent (Variables|Default|GetPhysicsHandle))
      (Variables|Default|SetIs_Vsat? false)
      (else
        (bind (_outhit _returnvalue_2) (Collision|LineTraceByChannel _returnvalue (+ _returnvalue (* (Math|Vector|GetForwardVector _camera) 1000)) "TraceTypeQuery1" false 0 "ForDuration"))
        (if _returnvalue_2
          (if (Physics|IsSimulatingPhysics (.HitComponent (Collision|BreakHitResult _outhit)) "None")
            (Class|PhysicsHandleComponent|GrabComponentatLocation (Variables|Default|GetPhysicsHandle) (.HitComponent (Collision|BreakHitResult _outhit)) "None" (Transformation|GetWorldLocation (.HitComponent (Collision|BreakHitResult _outhit))))
            (Physics|AddImpulse (.HitComponent (Collision|BreakHitResult _outhit)) "0.000000,0.100000,0.000000" "None" false)
            (Variables|Default|SetIs_Vsat? true)))))))

(fn ConstructionScript
  (|CallParentFunction))