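; DP_Stamina is a pawn Blueprint that manages sprint stamina on Left Shift.
; Pressing Shift starts a looping timer that drains Stamina and, through a DoOnce, calls StartSprint and stops regeneration.
; Releasing it clears that timer, calls FinishSprint and starts a looping timer that refills Stamina up to a cap.
; Depletion also ends the sprint, zeroes Stamina and resets the DoOnce, which Shift release leaves untouched.
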(event Custom|MinusStamina
  (if (> (Variables|Default|GetStamina) 0.0)
    (Variables|Default|SetStamina (- (Variables|Default|GetStamina) 0.1))
    (Utilities|FlowControl|DoOnce false :!label _label
      (:Completed
        (CallFunction|StartSprint)
        (CallFunction|StopTimerRegeneration)))
    (else
      (CallFunction|StopTimerSprint)
      (Variables|Default|SetStamina 0.0)
      (goto _label Reset))))

(event Custom|reg_st
  (if (> 0.0 (Variables|Default|GetStamina))
    (Variables|Default|SetStamina 0.0)
    (Utilities|FlowControl|DoOnce false) ; enters at Reset
    (elif (> (Variables|Default|GetStamina) 1e+01)
      (Variables|Default|SetStamina 1e+01)
      (else
        (Variables|Default|SetStamina (+ (Variables|Default|GetStamina) 0.1))))))

(event EventBeginPlay
  (|CallParentFunction) ; This node is disabled and will not be called.\nDrag off pins to build functionality.
)

(event Collision|EventActorBeginOverlap
  (params (OtherActor :type Actor%20Object%20Reference))
  (|CallParentFunction OtherActor) ; This node is disabled and will not be called.\nDrag off pins to build functionality.
)

(event EventTick
  (params (DeltaSeconds :type Float%20%28single-precision%29))
  (|CallParentFunction DeltaSeconds) ; This node is disabled and will not be called.\nDrag off pins to build functionality.
)

(event Input|KeyboardEvents|LeftShift
  (params (Key :type Key%20Structure :default "None"))
  (:Pressed
    (bind _returnvalue (Utilities|Time|SetTimerbyEvent (delegate Custom|MinusStamina) 0.1 true))
    (Variables|Default|SetSprintTimer _returnvalue))
  (:Released
    (CallFunction|StopTimerSprint)
    (bind _returnvalue_2 (Utilities|Time|SetTimerbyEvent (delegate Custom|reg_st) 0.1 true))
    (Variables|Default|SetRegenerationTimer _returnvalue_2)))

(fn ConstructionScript
  (|CallParentFunction))

(fn StopTimerSprint
  (Utilities|Time|ClearandInvalidateTimerbyHandle (Variables|Default|GetSprintTimer))
  (CallFunction|FinishSprint))

(fn StopTimerRegeneration
  (Utilities|Time|ClearandInvalidateTimerbyHandle (Variables|Default|GetRegenerationTimer))
  (return))