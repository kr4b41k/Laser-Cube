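; Player controller Blueprint that manages on-screen UI widgets and creates the cursor widget at BeginPlay.
; PC_Add_Widget works as a toggle: a widget already in the AllWidget list is removed, otherwise it is recorded and added to the viewport.
; PC_Remove_Widget takes listed widgets off screen, or prints an error label through PC_Eror, which ignores its detail text.
; PC_Game_Over pauses the game and shows the game-over widget through the same add path.
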(event EventBeginPlay
  (|CallParentFunction)
  (bind _returnvalue (UserInterface|CreateWidget "/Game/BluePrints/HUD/WB_Cursor.WB_Cursor_C"))
  (UserInterface|Viewport|AddtoViewport _returnvalue 0))

(event EventTick
  (params (DeltaSeconds :type Float%20%28single-precision%29))
  (|CallParentFunction DeltaSeconds) ; This node is disabled and will not be called.\nDrag off pins to build functionality.
)

(fn ConstructionScript
  (|CallParentFunction))

(fn PCEror
  (params (Name_Eror :type String) (Eror :type String))
  (Development|PrintString (Utilities|String|Append Name_Eror " Eror: ")))

(fn PCAddWidget
  (params (User_widget :type User%20Widget%20Object%20Reference))
  (LocalVariables|SetCurrent_WB User_widget)
  (if (Utilities|Array|ContainsItem (Variables|Default|GetAll_Widget) (LocalVariables|GetCurrent_WB))
    (CallFunction|PCRemoveWidget (LocalVariables|GetCurrent_WB))
    (return false)
    (else
      (Utilities|Array|AddUnique (Variables|Default|GetAll_Widget) (LocalVariables|GetCurrent_WB))
      (UserInterface|Viewport|AddtoViewport (LocalVariables|GetCurrent_WB) 0)
      (return true))))

(fn PCGameOver
  (Game|SetGamePaused true)
  (bind _returnvalue (UserInterface|CreateWidget "/Game/BluePrints/User_Widget/WB_Game_Over/WB_Game_Over.WB_Game_Over_C"))
  (CallFunction|PCAddWidget _returnvalue)
  (return true))

(fn PCRemoveWidget
  (params (User_Widget :type User%20Widget%20Object%20Reference))
  (LocalVariables|SetCureent_Remove_WB User_Widget)
  (if (Utilities|Array|ContainsItem (Variables|Default|GetAll_Widget) (LocalVariables|GetCureent_Remove_WB))
    (Utilities|Array|RemoveItem (Variables|Default|GetAll_Widget) (LocalVariables|GetCureent_Remove_WB))
    (Widget|RemovefromParent (LocalVariables|GetCureent_Remove_WB))
    (return true)
    (else
      (CallFunction|PCEror "Pc_Remove_vidget" "нет удаляемого виджета")
      (return false))))