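; PC_Laser_logic is a hub that links color-coded puzzle elements: buttons, lasers, laser targets, doors, lifts and stairs.
; Ini functions register each element in per-type arrays without duplicates.
; ACT and DACT functions loop over lasers, doors, lifts or stairs and send on or off interface messages to those matching the given or button-read color.
; Laser target functions instead add or remove the laser's color on the passed target.
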(event EventBeginPlay
  (|CallParentFunction) ; This node is disabled and will not be called.\nDrag off pins to build functionality.
)

(event EventTick
  (params (DeltaSeconds :type Float%20%28single-precision%29))
  (|CallParentFunction DeltaSeconds) ; This node is disabled and will not be called.\nDrag off pins to build functionality.
)

(fn ConstructionScript
  (|CallParentFunction))

(fn ACTDoor
  (params (SelfColor :type E_Color_Button%20Enum :default "NewEnumerator9"))
  (for _array_element (Variables|Default|GetALL_Door)
    (bind _color (Class|BPIDoorBase|GetDoorColor(Message) _array_element))
    (if (Utilities|Enum|Equal(Enum) _color SelfColor)
      (Class|BPIDoorBase|OpenDoor(Message) _array_element)))
  (return true))

(fn ACTLaser
  (params (Button_Self :type Actor%20Object%20Reference) (IsButtonPoint :type Boolean) (SelfColor :type E_Color_Button%20Enum :default "NewEnumerator9"))
  (if IsButtonPoint
    (LocalVariables|SetLocal_Color_Tags SelfColor)
    (else
      (bind _collor_tags (Class|BPIAButtonBase|GetColorButtonTags(Message) Button_Self))
      (LocalVariables|SetLocal_Color_Tags _collor_tags)))
  (for _array_element (Variables|Default|GetALL_Lasers)
    (bind _color_tags (Class|BPIALaserBase|GetColorLaserTags(Message) _array_element))
    (if (Utilities|Enum|Equal(Enum) _color_tags (LocalVariables|GetLocal_Color_Tags))
      (Class|BPIALaserBase|ACTLaser(Message) _array_element (LocalVariables|GetLocal_Color_Tags))))
  (return true))

(fn ACTLaserTarget
  (params (Laser_Self :type Actor%20Object%20Reference) (Laser_Target :type Actor%20Object%20Reference))
  (bind _color_tags (Class|BPIALaserBase|GetColorLaserTags(Message) Laser_Self))
  (Class|BPIALaserTargetBase|SetColorTagsLaserTarget(Message) Laser_Target _color_tags) ; задаем цвет лазероприемнику
  (return true))

(fn ACTLift
  (params (Color :type E_Color_Button%20Enum :default "NewEnumerator9"))
  (for _array_element (Variables|Default|GetALL_Lift)
    (bind _color (Class|BPILift|GetLiftColors(Message) _array_element))
    (if (Utilities|Enum|Equal(Enum) _color Color)
      (Class|BPILift|ActivatedLift(Message) _array_element)))
  (return true))

(fn ACTStairs
  (params (SelfColor :type E_Color_Button%20Enum :default "NewEnumerator9"))
  (for _array_element (Variables|Default|GetALL_Stairs)
    (bind _color (Class|BPIStairs|GetStairsColors(Message) _array_element))
    (if (Utilities|Enum|Equal(Enum) _color SelfColor)
      (Class|BPIStairs|ActivatedStairs(Message) _array_element)))
  (return true))

(fn DACTDoor
  (params (SelfColor :type E_Color_Button%20Enum :default "NewEnumerator9"))
  (for _array_element (Variables|Default|GetALL_Door)
    (bind _color (Class|BPIDoorBase|GetDoorColor(Message) _array_element))
    (if (Utilities|Enum|Equal(Enum) _color SelfColor)
      (Class|BPIDoorBase|ClosedDoor(Message) _array_element)))
  (return true))

(fn DACTLaser
  (params (Button_Self :type Actor%20Object%20Reference) (IsButtonPoint? :type Boolean) (Color :type E_Color_Button%20Enum :default "NewEnumerator9"))
  (if IsButtonPoint?
    (LocalVariables|SetLocal_Color_Tags Color)
    (else
      (bind _collor_tags (Class|BPIAButtonBase|GetColorButtonTags(Message) Button_Self))
      (LocalVariables|SetLocal_Color_Tags _collor_tags)))
  (for _array_element (Variables|Default|GetALL_Lasers)
    (bind _color_tags (Class|BPIALaserBase|GetColorLaserTags(Message) _array_element))
    (if (Utilities|Enum|Equal(Enum) _color_tags (LocalVariables|GetLocal_Color_Tags))
      (Class|BPIALaserBase|DACTLaser(Message) _array_element (LocalVariables|GetLocal_Color_Tags))))
  (return true))

(fn DACTLaserTarget
  (params (Laser_Self :type Actor%20Object%20Reference) (Laser_Target :type Actor%20Object%20Reference))
  (bind _color_tags (Class|BPIALaserBase|GetColorLaserTags(Message) Laser_Self))
  (Class|BPIALaserTargetBase|RemoveColorTagsLaserTarget(Message) Laser_Target _color_tags)
  (return true))

(fn DACTLift
  (params (Color :type E_Color_Button%20Enum :default "NewEnumerator9"))
  (for _array_element (Variables|Default|GetALL_Lift)
    (bind _color (Class|BPILift|GetLiftColors(Message) _array_element))
    (if (Utilities|Enum|Equal(Enum) _color Color)
      (Class|BPILift|DeActivatedLift(Message) _array_element)))
  (return true))

(fn DACTStairs
  (params (Color :type E_Color_Button%20Enum :default "NewEnumerator9"))
  (for _array_element (Variables|Default|GetALL_Stairs)
    (bind _color (Class|BPIStairs|GetStairsColors(Message) _array_element))
    (if (Utilities|Enum|Equal(Enum) _color Color)
      (Class|BPIStairs|DeActivatedStairs(Message) _array_element)))
  (return true))

(fn IniButton
  (params (A_Button :type Actor%20Object%20Reference))
  (LocalVariables|SetLocal_Button A_Button)
  (Utilities|Array|AddUnique (Variables|Default|GetALL_Button) (LocalVariables|GetLocal_Button))
  (return true))

(fn IniDoor
  (params (A_Door :type Actor%20Object%20Reference))
  (LocalVariables|SetLocal_Door A_Door)
  (Utilities|Array|AddUnique (Variables|Default|GetALL_Door) (LocalVariables|GetLocal_Door))
  (return true))

(fn IniLaser
  (params (A_Laser :type Actor%20Object%20Reference))
  (LocalVariables|SetLocal_lasers A_Laser)
  (Utilities|Array|AddUnique (Variables|Default|GetALL_Lasers) (LocalVariables|GetLocal_lasers))
  (return true))

(fn IniLaserTarget
  (params (A_Laser_Target :type Actor%20Object%20Reference))
  (LocalVariables|SetLocal_Laser_Target A_Laser_Target)
  (Utilities|Array|AddUnique (Variables|Default|GetALL_Laser_Target) (LocalVariables|GetLocal_Laser_Target))
  (return true))

(fn IniLift
  (params (Lift :type Actor%20Object%20Reference))
  (bind _output_get (LocalVariables|SetLocalLift Lift))
  (Utilities|Array|AddUnique (Variables|Default|GetALL_Lift) _output_get)
  (return true))

(fn IniStairs
  (params (Stairs :type Actor%20Object%20Reference))
  (bind _output_get (LocalVariables|SetLocalStairs Stairs))
  (Utilities|Array|AddUnique (Variables|Default|GetALL_Stairs) _output_get)
  (return true))